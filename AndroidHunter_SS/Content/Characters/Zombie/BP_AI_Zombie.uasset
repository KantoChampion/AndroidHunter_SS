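; Zombie enemy character that wanders at random, chases the player and explodes when its health runs out.
; Tick checks a Sight component's overlap, then either moves to the player or calls Patrol, which picks random reachable points after random delays and re-calls itself.
; Each hit decrements health, plays a reaction animation and briefly swaps a material.
; Animations are set directly on the mesh; the pawn-sensing event is empty.
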(event OnSeePawn(PawnSensing)
  (params (Pawn :type Pawn%20Object%20Reference)))

(event OnComponentBeginOverlap(Sight)
  (params (OverlappedComponent :type Primitive%20Component%20Object%20Reference) (OtherActor :type Actor%20Object%20Reference) (OtherComp :type Primitive%20Component%20Object%20Reference) (OtherBodyIndex :type Integer) (bFromSweep :type Boolean) (SweepResult :type Hit%20Result%20Structure%20%28by%20ref%29)))

(event Custom|Patrol
  (bind _returnvalue (Transformation|GetActorLocation))
  (bind _mesh (Variables|Character|GetMesh))
  (bind _randomlocation (AI|Navigation|GetRandomReachablePointinRadius (Math|Vector|MakeVector (.x _returnvalue) (.y _returnvalue) (.z _returnvalue)) 1e+03 0 0))
  (if (and (not (Variables|Default|GetcanSeeEnemy)) (not (Variables|Default|GetbTakeDamage)))
    (Variables|Default|SetisMoving true)
    (Utilities|FlowControl|Delay (Math|Random|RandomFloatinRange 0.5 6.0))
    (AI|AIMoveTo self (Math|Vector|MakeVector (.x _randomlocation) (.y _randomlocation) (.z _returnvalue)) 0 5.0 false
      (:then
        (Components|Animation|SetAnimation _mesh "/Game/Characters/Zombie/Zombie_Run_Anim_mixamo_com.Zombie_Run_Anim_mixamo_com")
        (Audio|Components|Audio|Play _mesh true))
      (:OnSuccess
        (Variables|Default|SetisMoving false :!label _label)
        (Components|Animation|SetAnimation _mesh "/Game/Characters/Zombie/Zombie_Idle_mixamo_com.Zombie_Idle_mixamo_com")
        (CallFunction|Patrol)
        (Audio|Components|Audio|Play _mesh true))
      (:OnFail
        (goto _label)))))

(event Custom|TakeDamage
  (CallFunction|SetHurt)
  (bind _result (Math|Float|DecrementFloat (Variables|Default|GetHealth))
    (:%20%20
      (Variables|Default|SetHealth _result)
      (if (== (Variables|Default|GetHealth) 0.0)
        (Effects|SpawnEmitteratLocation "/Game/StarterContent/Particles/P_Explosion.P_Explosion" (Transformation|GetWorldLocation (Variables|Collision|GetCapsuleComponent)) "0, 0, 0" "2.000000,2.000000,2.000000")
        (Actor|DestroyActor)
        (else
          (Rendering|Material|SetMaterial (Variables|Character|GetMesh) 1 "/Game/Characters/Zombie/M_TakeDamage.M_TakeDamage")
          (Development|PrintString "TOOK DAMAGE 
")
          (Utilities|FlowControl|Delay (Variables|Default|GetDam_MaterialDuration))
          (Rendering|Material|SetMaterial (Variables|Character|GetMesh) 1 "/Game/Characters/Zombie/Beta_HighLimbsGeoSG2.Beta_HighLimbsGeoSG2"))))))

(event Custom|Set%20Running
  (bind _mesh (Variables|Character|GetMesh))
  (Components|Animation|SetAnimation _mesh "/Game/Characters/Zombie/Zombie_Run_Anim_mixamo_com.Zombie_Run_Anim_mixamo_com")
  (Audio|Components|Audio|Play _mesh true))

(event Custom|Set%20Idle
  (bind _mesh (Variables|Character|GetMesh))
  (Components|Animation|SetAnimation _mesh "/Game/Characters/Zombie/Zombie_Run_Anim_Take_001.Zombie_Run_Anim_Take_001")
  (Audio|Components|Audio|Play _mesh true))

(event Custom|Set%20Hurt
  (bind _mesh (Variables|Character|GetMesh))
  (Variables|Default|SetbTakeDamage true)
  (Components|Animation|SetAnimation _mesh "/Game/Characters/Zombie/Zombie_Reaction_Hit_mixamo_com.Zombie_Reaction_Hit_mixamo_com")
  (Audio|Components|Audio|Play _mesh true)
  (Utilities|FlowControl|Delay 0.8)
  (Variables|Default|SetbTakeDamage false))

(event EventBeginPlay)

(event Collision|EventActorBeginOverlap
  (params (OtherActor :type Actor%20Object%20Reference)))

(event EventTick
  (params (DeltaSeconds :type Float%20%28single-precision%29))
  (bind _asbp_third_person_character (Utilities|Casting|CastToBP_ThirdPersonCharacter (Game|GetPlayerCharacter 0)))
  (if (Collision|IsOverlappingActor (Variables|Default|GetSight) 0 :!class /Script/Engine.PrimitiveComponent)
    (Variables|Default|SetcanSeeEnemy true)
    (if (Variables|Default|GetcanSeeEnemy)
      (AI|AIMoveTo self "0, 0, 0" _asbp_third_person_character 5.0 false
        (:then
          (Utilities|FlowControl|DoOnce false :!label _label
            (:Completed
              (CallFunction|SetRunning))))
        (:OnFail
          (goto _label Reset))))
    (else
      (Variables|Default|SetcanSeeEnemy false)
      (CallFunction|Patrol))))

(fn ConstructionScript)