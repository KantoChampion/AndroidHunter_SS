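; BP_Projectile1 is a projectile actor that damages BP_AI_Zombie characters on impact.
; On hit, it simply destroys itself if the struck component simulates physics.
; Otherwise, a hit on a zombie spawns an explosion emitter at its Sphere, calls the zombie's TakeDamage and destroys the projectile.
; Other hits leave it alive, and the physics impulse node is disconnected, so it never runs.
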(event EventBeginPlay)

(event Collision|EventHit
  (params (MyComp :type Primitive%20Component%20Object%20Reference) (Other :type Actor%20Object%20Reference) (OtherComp :type Primitive%20Component%20Object%20Reference) (bSelfMoved :type Boolean) (HitLocation :type Vector :default "0, 0, 0") (HitNormal :type Vector :default "0, 0, 0") (NormalImpulse :type Vector :default "0, 0, 0") (Hit :type Hit%20Result%20Structure%20%28by%20ref%29))
  (if (Physics|IsSimulatingPhysics OtherComp "None")
    (Actor|DestroyActor)
    (else
      (bind _asbp_ai_zombie (Utilities|Casting|CastToBP_AI_Zombie Other))
      (if (Utilities|IsValid _asbp_ai_zombie)
        (Effects|SpawnEmitteratLocation "/Game/StarterContent/Particles/P_Explosion.P_Explosion" (Transformation|GetWorldLocation (Variables|Default|GetSphere)))
        (Default|TakeDamage _asbp_ai_zombie)
        (Actor|DestroyActor)))))

(fn ConstructionScript)